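; Actor component that manages an SCharacterBase owner's talents through the Gameplay Ability System.
; Spending a point through its server event either grants a new talent, giving its abilities and applying its effects, or levels it up to its maximum level at most.
; Ability and effect handles are stored per talent so level-ups can update them in place.
; The GrantedTalents list tracks levels, and its OnRep fires a talent-changed notification.
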(event `self.ReceiveBeginPlay`
  (bind _asscharacter_base (cast `SCharacterBase` (`self.GetOwner`)))
  (bind _output_get (set `self.OwnerCharacter` _asscharacter_base))
  (set `self.OwnerASC` (`AbilitySystemBlueprintLibrary.GetAbilitySystemComponent` _output_get)))

(event `Server_SpendPointOnTalent`
  (params (Talent :type "/Game/GameplayAbilitySystem/Talents/Types/PDA_Talent Object Reference"))
  (bind (_success _grantedtalent) (`self.FindGrantedTalent` Talent))
  (if _success
    (`self.LevelUpGrantedTalent` _grantedtalent)
    (else
      (`self.GrantTalent` Talent 1))))

(fn `ApplyGameplayEffectsToOwner`
  (params (Effects :type "Array of GameplayEffect Class Reference") (Level :type Integer) (Talent :type "/Game/GameplayAbilitySystem/Talents/Types/PDA_Talent Object Reference (by ref)"))
  (locals (AppliedEffectHandles :type "Array of ActiveGameplayEffectHandle Structure"))
  (for _array_element Effects
    (bind _returnvalue (`AbilitySystemComponent.BP_ApplyGameplayEffectToSelf` :`self` (`self.OwnerASC`) :`GameplayEffectClass` _array_element :`Level` (`KismetMathLibrary.Conv_IntToDouble` Level)))
    (`KismetArrayLibrary.Array_AddUnique` (`local.AppliedEffectHandles`) _returnvalue))
  (`BlueprintMapLibrary.Map_Add` (`self.EffectHandlesApplyedByTalent`) Talent (make `/Game/GameplayAbilitySystem/Talents/Types/S_TalentEffectsHandles` (`local.AppliedEffectHandles`))))

(fn `FindGrantedTalent`
  (params (Talent :type "/Game/GameplayAbilitySystem/Talents/Types/PDA_Talent Object Reference"))
  (returns (Success :type Boolean) (GrantedTalent :type "/Game/GameplayAbilitySystem/Talents/Types/S_GrantedTalent Structure"))
  (for _array_element (`self.GrantedTalents`)
    (if (== (`.Talent_3_617339944EB6B1FB018F2DA51E8DFB4F` (break `/Game/GameplayAbilitySystem/Talents/Types/S_GrantedTalent` _array_element)) (`local.Talent`))
      (return true _array_element)))
  (return false))

(fn `GiveAbilitiesToOwner`
  (params (Abilities :type "Array of SGameplayAbility Class Reference") (Level :type Integer) (Talent :type "/Game/GameplayAbilitySystem/Talents/Types/PDA_Talent Object Reference (by ref)"))
  (bind _returnvalue (`SCharacterBase.GrantAbilities` (`self.OwnerCharacter`) Abilities Level))
  (`BlueprintMapLibrary.Map_Add` (`self.AbilitySpecHandlesGrantedByTalent`) (`local.Talent`) (make `/Game/GameplayAbilitySystem/Talents/Types/S_TalentAbilitySpecHandles` _returnvalue)))

(fn `GrantTalent`
  (params (Talent :type "/Game/GameplayAbilitySystem/Talents/Types/PDA_Talent Object Reference") (StartingLevel :type Integer))
  (returns (Success :type Boolean))
  (locals (ClampedLevel :type Integer))
  (bind _grantedtalents (`self.GrantedTalents`))
  (bind _success (`self.FindGrantedTalent` Talent))
  (if _success
    (return false)
    (else
      (set `local.ClampedLevel` (`KismetMathLibrary.Clamp` (`local.StartingLevel`) 1 (`/Game/GameplayAbilitySystem/Talents/Types/PDA_Talent.MaxLevel` (`local.Talent`))))
      (`self.GiveAbilitiesToOwner` (`/Game/GameplayAbilitySystem/Talents/Types/PDA_Talent.AbilityToGrant` (`local.Talent`)) (`local.ClampedLevel`) (`local.Talent`))
      (`self.ApplyGameplayEffectsToOwner` (`/Game/GameplayAbilitySystem/Talents/Types/PDA_Talent.EffectsToApply` (`local.Talent`)) (`local.ClampedLevel`) (`local.Talent`))
      (`KismetArrayLibrary.Array_Add` _grantedtalents (make `/Game/GameplayAbilitySystem/Talents/Types/S_GrantedTalent` (`local.Talent`) (`local.ClampedLevel`)))
      (set `self.GrantedTalents` _grantedtalents)
      (return true))))

(fn `IncrementedGrantedTalentLevel`
  (params (GrantedTalent :type "/Game/GameplayAbilitySystem/Talents/Types/S_GrantedTalent Structure"))
  (bind (_talent _level) (break `/Game/GameplayAbilitySystem/Talents/Types/S_GrantedTalent` GrantedTalent))
  (bind _grantedtalents (`self.GrantedTalents`))
  (`KismetArrayLibrary.Array_AddUnique` _grantedtalents (make `/Game/GameplayAbilitySystem/Talents/Types/S_GrantedTalent` _talent (+ _level 1)))
  (`KismetArrayLibrary.Array_RemoveItem` _grantedtalents (`local.GrantedTalent`))
  (set `self.GrantedTalents` _grantedtalents))

(fn `LevelUpGrantedTalent`
  (params (GrantedTalent :type "/Game/GameplayAbilitySystem/Talents/Types/S_GrantedTalent Structure"))
  (returns (Success :type Boolean))
  (bind (_talent _level) (break `/Game/GameplayAbilitySystem/Talents/Types/S_GrantedTalent` GrantedTalent))
  (bind _talent_2 (break `/Game/GameplayAbilitySystem/Talents/Types/S_GrantedTalent` (`local.GrantedTalent`)))
  (if (> (`/Game/GameplayAbilitySystem/Talents/Types/PDA_Talent.MaxLevel` _talent) _level)
    (`self.IncrementedGrantedTalentLevel` (`local.GrantedTalent`))
    (`self.SetLevelOfAbilitiesGrantedByTalent` _talent_2)
    (`self.SetLevelOfEffectsApplyedByTalent` _talent_2)
    (return true)
    (else
      (return false))))

(fn `OnRep_GrantedTalents`
  (`self.OnTalentChanged`))

(fn `SetLevelOfAbilitiesGrantedByTalent`
  (params (Talent :type "/Game/GameplayAbilitySystem/Talents/Types/PDA_Talent Object Reference"))
  (bind (_success _grantedtalent) (`self.FindGrantedTalent` Talent))
  (for _array_element (`.SpecHandles_3_4426A4F64A3E0F14AE9FCBB5E70C41D9` (break `/Game/GameplayAbilitySystem/Talents/Types/S_TalentAbilitySpecHandles` (`BlueprintMapLibrary.Map_Find` (`self.AbilitySpecHandlesGrantedByTalent`) Talent)))
    (bind _assgameplay_ability (cast `SGameplayAbility` (`.ReturnValue` (`AbilitySystemBlueprintLibrary.GetGameplayAbilityFromSpecHandle` (`self.OwnerASC`) _array_element))))
    (`SGameplayAbility.SetAbilityLevel` _assgameplay_ability (`.Level_5_BC58BEE94FC43FF8076FC8B85128E6BC` (break `/Game/GameplayAbilitySystem/Talents/Types/S_GrantedTalent` _grantedtalent)))))

(fn `SetLevelOfEffectsApplyedByTalent`
  (params (GrantedTalent :type "/Game/GameplayAbilitySystem/Talents/Types/PDA_Talent Object Reference"))
  (bind (_success _grantedtalent) (`self.FindGrantedTalent` GrantedTalent))
  (for _array_element (`.EffectsHandles_3_A62BD4634261BC15A4EF26846D649719` (break `/Game/GameplayAbilitySystem/Talents/Types/S_TalentEffectsHandles` (`BlueprintMapLibrary.Map_Find` (`self.EffectHandlesApplyedByTalent`) GrantedTalent)))
    (`AbilitySystemComponent.SetActiveGameplayEffectLevel` (`self.OwnerASC`) _array_element (`.Level_5_BC58BEE94FC43FF8076FC8B85128E6BC` (break `/Game/GameplayAbilitySystem/Talents/Types/S_GrantedTalent` _grantedtalent)))))