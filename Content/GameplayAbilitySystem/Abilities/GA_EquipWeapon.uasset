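; GA_EquipWeapon is a Gameplay Ability that equips or unequips the avatar's weapon when triggered by a gameplay event.
; It commits, finds the BP_WeaponManager component on the avatar, and switches on the first target tag of the event to equip the staff or axe weapon class.
; An unrecognized or missing tag unequips instead, and the ability then ends.
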(event `self.K2_ActivateAbilityFromEvent`
  (params (EventData :type "GameplayEventData Structure (by ref)"))
  (bind _gameplaytags (`BlueprintGameplayTagLibrary.BreakGameplayTagContainer` (`.TargetTags` (break `GameplayEventData` EventData))))
  (`|ExecutionSequence`
    (:`then_0`
      (`self.K2_CommitAbility`)
      (bind _returnvalue (`Actor.GetComponentByClass` (`self.GetAvatarActorFromActorInfo`) "/Game/Weapons/BP_WeaponManager.BP_WeaponManager_C"))
      (`/Engine/EditorBlueprintResources/StandardMacros.IsValid` _returnvalue
        (:`Is Valid`
          (if (`KismetArrayLibrary.Array_IsNotEmpty` _gameplaytags)
            (`|SwitchGameplayTag` (`|GetArrayItem` _gameplaytags)
              (:`Default`
                (`/Game/Weapons/BP_WeaponManager.UnequipWeapon` _returnvalue))
              (:`Weapon.Ranged.Staff`
                (`/Game/Weapons/BP_WeaponManager.EquipWeapon` _returnvalue "/Game/Weapons/BP_Weapon_Staff.BP_Weapon_Staff_C"))
              (:`Weapon.Melee.Axe`
                (`/Game/Weapons/BP_WeaponManager.EquipWeapon` _returnvalue "/Game/Weapons/BP_Weapon_Axe.BP_Weapon_Axe_C")))
            (else
              (`/Game/Weapons/BP_WeaponManager.UnequipWeapon` _returnvalue))))))
    (:`then_1`
      (`self.K2_EndAbility`))))