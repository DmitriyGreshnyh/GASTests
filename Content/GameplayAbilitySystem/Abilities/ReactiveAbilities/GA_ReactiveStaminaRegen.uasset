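; Reactive gameplay ability that manages delayed stamina regeneration on its avatar.
; It watches an attribute for changes and compares each new value with the cached previous one.
; A drop removes the active GE_Status_StaminaRegen and reapplies it after a short delay, without cancelling delays already pending.
; Otherwise, it removes the effect by stored handle once the value reaches a second attribute reading, presumably the maximum.
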(event `self.K2_ActivateAbility`
  (set `self.OldStamina` (`.ReturnValue` (`AbilitySystemBlueprintLibrary.GetFloatAttribute` (`self.GetAvatarActorFromActorInfo`) (struct :`AttributeName` "Stamina" :`Attribute` "/Script/GASTests.SBasicAttributeSet:Stamina" :`AttributeOwner` "/Script/CoreUObject.Class'/Script/GASTests.SBasicAttributeSet'"))))
  (`AbilityTask_WaitAttributeChange.WaitForAttributeChange` (struct :`AttributeName` "Stamina" :`Attribute` "/Script/GASTests.SBasicAttributeSet:Stamina" :`AttributeOwner` "/Script/CoreUObject.Class'/Script/GASTests.SBasicAttributeSet'") (struct) (struct) false null
    (:`OnChange`
      (`|ExecutionSequence`
        (:`then_0`
          (bind _output_get (set `self.NewStamina` (`.ReturnValue` (`AbilitySystemBlueprintLibrary.GetFloatAttribute` (`self.GetAvatarActorFromActorInfo`) (struct :`AttributeName` "Stamina" :`Attribute` "/Script/GASTests.SBasicAttributeSet:Stamina" :`AttributeOwner` "/Script/CoreUObject.Class'/Script/GASTests.SBasicAttributeSet'")))))
          (if (< _output_get (`self.OldStamina`))
            (`self.BP_RemoveGameplayEffectFromOwnerWithHandle` (`self.StaminaRegenEffectHandle`))
            (`AbilityTask_WaitDelay.WaitDelay` 1.0
              (:`OnFinish`
                (bind _returnvalue (`self.BP_ApplyGameplayEffectToOwner` "/Game/GameplayAbilitySystem/Effects/GE_Status_StaminaRegen.GE_Status_StaminaRegen_C"))
                (set `self.StaminaRegenEffectHandle` _returnvalue)))
            (elif (>= (`self.NewStamina`) (`.ReturnValue` (`AbilitySystemBlueprintLibrary.GetFloatAttribute` (`self.GetAvatarActorFromActorInfo`) (struct :`AttributeName` "Stamina" :`Attribute` "/Script/GASTests.SBasicAttributeSet:Stamina" :`AttributeOwner` "/Script/CoreUObject.Class'/Script/GASTests.SBasicAttributeSet'"))))
              (`self.BP_RemoveGameplayEffectFromOwnerWithHandle` (`self.StaminaRegenEffectHandle`)))))
        (:`then_1`
          (set `self.OldStamina` (`self.NewStamina`)))))))