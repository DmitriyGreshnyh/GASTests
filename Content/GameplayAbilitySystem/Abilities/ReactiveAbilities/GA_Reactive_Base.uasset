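; Base reactive gameplay ability that turns stacked debuffs the owner applies into a status effect on the target.
; On activation it listens for effects applied to targets, checking each against the status effect data asset's debuff tag and max stack count.
; When stacks exceed the max, it applies the asset's effect with the configured duration, first passing the spec through ModifyEffectSpecBeforeApplication, a pass-through hook.
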(event `self.K2_ActivateAbility`
  (bind (_asynctaskproxy _target _spechandle _activehandle) (`AbilityTask_WaitGameplayEffectApplied_Target.WaitGameplayEffectAppliedToTarget` (struct) (struct) (struct) (struct) (struct) false null)
    (:`OnApplied`
      (bind _returnvalue (`AbilitySystemBlueprintLibrary.GetGameplayEffectFromActiveEffectHandle` _activehandle))
      (`/Engine/EditorBlueprintResources/StandardMacros.IsValid` _returnvalue
        (:`Is Valid`
          (if (`GameplayTagAssetInterface.HasMatchingGameplayTag` _returnvalue (`/Game/GameplayAbilitySystem/Data/PDA_StatusEffect.Debuff Tag` (`self.DA_StatusEffect`)))
            (bind _returnvalue_2 (`AbilitySystemBlueprintLibrary.GetActiveGameplayEffectStackCount` _activehandle))
            (if (> _returnvalue_2 (`/Game/GameplayAbilitySystem/Data/PDA_StatusEffect.Max Stack Count` (`self.DA_StatusEffect`)))
              (bind _returnvalue_3 (`AbilitySystemBlueprintLibrary.SetDuration` (`self.MakeOutgoingGameplayEffectSpec` (`/Game/GameplayAbilitySystem/Data/PDA_StatusEffect.Gameplay Effect to Apply` (`self.DA_StatusEffect`))) (`/Game/GameplayAbilitySystem/Data/PDA_StatusEffect.Status Duration` (`self.DA_StatusEffect`))))
              (bind _returnvalue_4 (`self.ModifyEffectSpecBeforeApplication` _returnvalue_3))
              (`self.K2_ApplyGameplayEffectSpecToTarget` _returnvalue_4 (`AbilitySystemBlueprintLibrary.AbilityTargetDataFromActor` _target)))))))))

(fn `ModifyEffectSpecBeforeApplication`
  (params (SpecHandle :type "GameplayEffectSpecHandle Structure"))
  (returns (ReturnValue :type "GameplayEffectSpecHandle Structure"))
  (return SpecHandle))