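; Base melee attack gameplay ability that plays an attack montage with the equipped weapon from the avatar's weapon manager.
; On authority, gameplay events for hit scan start and end toggle the weapon's hit scan, passing it a damage effect spec with SetByCaller magnitude.
; Montage completion or interruption ends the ability, which also stops the hit scan; child abilities can override a montage-started hook.
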(event `self.K2_ActivateAbility`
  (bind _returnvalue (`Actor.GetComponentByClass` (`self.GetAvatarActorFromActorInfo`) "/Game/Weapons/BP_WeaponManager.BP_WeaponManager_C"))
  (`/Engine/EditorBlueprintResources/StandardMacros.IsValid` _returnvalue
    (:`Is Valid`
      (set `self.Equipped Weapon` (`/Game/Weapons/BP_WeaponManager.GetEquippedWeapon` _returnvalue))
      (`self.Equipped Weapon`
        (:`then`
          (bind _attackmontage (`self.AttackMontage`)
            (:`then`
              (`AbilityTask_PlayMontageAndWait.CreatePlayMontageAndWaitProxy` "None" _attackmontage 1.0 "None" true 1.0 0.0 true
                (:`then`
                  (`self.MontageStarted`)
                  (`self.K2_HasAuthority`
                    (:`True`
                      (`AbilityTask_WaitGameplayEvent.WaitGameplayEvent` (struct :`TagName` "Events.HitScan.Start") null
                        (:`then`
                          (`AbilityTask_WaitGameplayEvent.WaitGameplayEvent` (struct :`TagName` "Events.HitScan.End") null
                            (:`EventReceived`
                              (`self.HandleHitScanEnd`))))
                        (:`EventReceived`
                          (`self.HandleHitScanStart`))))))
                (:`OnCompleted`
                  (`self.K2_EndAbility` :!label _label))
                (:`OnInterrupted`
                  (goto _label))
                (:`OnCancelled`
                  (goto _label))))
            (:`else`
              (`self.K2_EndAbility`))))
        (:`else`
          (`self.K2_EndAbility` :!label _label_2))))
    (:`Is Not Valid`
      (goto _label_2))))

(event `HandleHitScanStart`
  (bind _equipped_weapon (`self.Equipped Weapon`)
    (:`then`
      (bind _returnvalue (`AbilitySystemBlueprintLibrary.AssignTagSetByCallerMagnitude` (`self.MakeOutgoingGameplayEffectSpec` (`self.DamageEffectClass`)) (struct :`TagName` "Data.Damage") (`self.DamageMagnitude`)))
      (`/Game/Weapons/BP_Weapon_Base.HitScanStart` _equipped_weapon _returnvalue))
    (:`else`)))

(event `HandleHitScanEnd`
  (bind _equipped_weapon (`self.Equipped Weapon`)
    (:`then`
      (`/Game/Weapons/BP_Weapon_Base.HitScanEnd` _equipped_weapon))
    (:`else`)))

(event `self.K2_OnEndAbility`
  (params (bWasCancelled :type Boolean))
  (`self.HandleHitScanEnd`))

(event `MontageStarted`
  ; For child overriding
)