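; Gameplay ability for a melee axe combo attack that chains hits within a single montage when input is timed correctly.
; On montage start it listens for gameplay events that open and close a combo window and register input.
; When the window closes without timely input the ability ends, though non-player-controlled users always continue.
; Each continued hit raises the combo count, which scales damage before the parent's hit scan runs.
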(event `self.K2_ActivateAbility`
  (`parent.K2_ActivateAbility`)
  (set `self.AlwaysContinueCombo` (not (`self.IsControlledByPlayer`))))

(event `self.K2_OnEndAbility`
  (params (bWasCancelled :type Boolean))
  (`parent.K2_OnEndAbility` bWasCancelled))

(event `self.MontageStarted`
  (set `self.ComboCount` 1)
  (`AbilityTask_WaitGameplayEvent.WaitGameplayEvent` (struct :`TagName` "Events.ContinueCombo.Start") null
    (:`then`
      (`AbilityTask_WaitGameplayEvent.WaitGameplayEvent` (struct :`TagName` "Events.ContinueCombo.End") null
        (:`then`
          (`AbilityTask_WaitGameplayEvent.WaitGameplayEvent` (struct :`TagName` "Events.ContinueCombo.Input") null
            (:`EventReceived`
              (if (`self.IsWithinComboWindow`)
                (set `self.RecievedInputAtRightTime` true)))))
        (:`EventReceived`
          (set `self.IsWithinComboWindow` false)
          (if (or (`self.RecievedInputAtRightTime`) (`self.AlwaysContinueCombo`))
            (set `self.RecievedInputAtRightTime` false)
            (`/Engine/EditorBlueprintResources/StandardMacros.IncrementInt` (`self.ComboCount`))
            (else
              (`self.K2_EndAbility`))))))
    (:`EventReceived`
      (set `self.IsWithinComboWindow` true)
      (set `self.RecievedInputAtRightTime` false))))

(event `self.HandleHitScanStart`
  (set `self.DamageMagnitude` (`KismetMathLibrary.Conv_IntToDouble` (* (`self.ComboCount`) -25)))
  (`parent.HandleHitScanStart`))