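; Gameplay Ability for an area-of-effect lightning strike that damages pawns around a chosen ground point.
; It uses the avatar's attack target, traced to the ground, or otherwise lets players confirm a decal ground-trace target during a looping montage.
; After commit, it shows an indicator cue and plays the trigger montage, whose gameplay event fires the strike cue and authority-only sphere-trace SetByCaller damage.
; Pressing input again cancels the ability.
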(event `self.K2_ActivateAbility`
  ; Phase 1
  (`self.WaitCancelInput`)
  (bind _attacktarget (message `/Game/GameplayAbilitySystem/BPI_Targeting.GetAttackTarget` (`self.GetAvatarActorFromActorInfo`)))
  (`/Engine/EditorBlueprintResources/StandardMacros.IsValid` _attacktarget
    (:`Is Valid`
      (set `self.ConfeirmedAOELocation` (`self.GetTargetGroundLocation` _attacktarget))
      (`self.ConfirmedStrike`))
    (:`Is Not Valid`
      (`self.StartTargeting`))))

(event `StartTargeting`
  ; Phase 1
  (if (`self.IsControlledByPlayer`)
    (`self.LoopTargetingAnimation`)
    (set `self.IsWaitingTargetData` true)
    (bind (_asynctaskproxy _data) (`AbilityTask_WaitTargetData.WaitTargetData` "None" "UserConfirmed" "/Game/GameplayAbilitySystem/TargetingACtors/GATargetACtor_GroundTrace_Decal.GATargetACtor_GroundTrace_Decal_C" (* (`self.AOERadius`) 2.0) "/Game/Decals/Decal_AOE.Decal_AOE" 0.0 0.0 2000.0 (struct :`Name` "NoCollision") true (`self.MakeTargetLocationInfoFromOwnerActor`) (struct) null)
      (:`ValidData`
        (set `self.IsWaitingTargetData` false)
        (set `self.ConfeirmedAOELocation` (`.Location` (`GameplayStatics.BreakHitResult` (`AbilitySystemBlueprintLibrary.GetHitResultFromTargetData` _data))))
        (`self.ConfirmedStrike`))
      (:`Cancelled`
        (set `self.IsWaitingTargetData` false)))
    (else
      (`self.K2_EndAbility`))))

(event `LoopTargetingAnimation`
  ; Phase 1
  (`AbilityTask_PlayMontageAndWait.CreatePlayMontageAndWaitProxy` "None" "/Game/Animations/Staff/AM_AOE_Targeting.AM_AOE_Targeting"
    (:`OnBlendOut`
      (if (`self.IsWaitingTargetData`)
        (`self.LoopTargetingAnimation`)))
    (:`OnInterrupted`
      (if (`self.IsWaitingTargetData`)
        (`self.K2_EndAbility`)))))

(event `ConfirmedStrike`
  ; Phase 2
  (bind _returnvalue (`self.K2_CommitAbility`))
  (if _returnvalue
    (`self.K2_AddGameplayCueWithParams` (struct :`TagName` "GameplayCue.AOEIndicator") (`AbilitySystemBlueprintLibrary.MakeGameplayCueParameters` 0.0 (* (`self.AOERadius`) 2.0) (struct) (struct) (struct) (struct) (struct) (`self.ConfeirmedAOELocation`)))
    (`AbilityTask_PlayMontageAndWait.CreatePlayMontageAndWaitProxy` "None" "/Game/Animations/Staff/AM_AOE_Trigger.AM_AOE_Trigger"
      (:`then`
        (`AbilityTask_WaitGameplayEvent.WaitGameplayEvent` (struct :`TagName` "Events.Montage.Triggered") null
          (:`EventReceived`
            (`self.K2_ExecuteGameplayCueWithParams` (struct :`TagName` "GameplayCue.LightingStrike") (`AbilitySystemBlueprintLibrary.MakeGameplayCueParameters` 0.0 0.0 (struct) (struct) (struct) (struct) (struct) (`self.ConfeirmedAOELocation`)))
            (`self.AOEDamage`)
            (`self.K2_RemoveGameplayCue` (struct :`TagName` "GameplayCue.AOEIndicator")))))
      (:`OnCompleted`
        (`self.K2_EndAbility` :!label _label))
      (:`OnInterrupted`
        (goto _label))
      (:`OnCancelled`
        (goto _label)))
    (else
      (`self.K2_EndAbility`))))

(event `AOEDamage`
  (bind _confeirmedaoelocation (`self.ConfeirmedAOELocation`))
  ; Phase 2
  (`self.K2_HasAuthority`
    (:`True`
      (bind _outhits (`KismetSystemLibrary.SphereTraceMultiForObjects` _confeirmedaoelocation _confeirmedaoelocation (`self.AOERadius`) (`|MakeArray` "ObjectTypeQuery3" :!type "EObjectTypeQuery Enum") false (`|MakeArray` (`self.GetAvatarActorFromActorInfo`)) "ForDuration"))
      (`KismetArrayLibrary.Array_Clear` (`self.HitActors`))
      (for _array_element _outhits
        (bind (_bblockinghit _binitialoverlap _time _distance _location _impactpoint _normal _impactnormal _physmat _hitactor) (`GameplayStatics.BreakHitResult` _array_element))
        (if (not (`KismetArrayLibrary.Array_Contains` (`self.HitActors`) _hitactor))
          (`KismetArrayLibrary.Array_AddUnique` (`self.HitActors`) _hitactor)
          (bind _returnvalue (`AbilitySystemBlueprintLibrary.GetAbilitySystemComponent` _hitactor))
          (`/Engine/EditorBlueprintResources/StandardMacros.IsValid` _returnvalue
            (:`Is Valid`
              (bind _returnvalue_2 (`AbilitySystemBlueprintLibrary.AssignTagSetByCallerMagnitude` (`self.MakeOutgoingGameplayEffectSpec` "/Game/GameplayAbilitySystem/Effects/GE_Damage_Instance.GE_Damage_Instance_C") (struct :`TagName` "Data.Damage") (`self.DamageMagnitude`)))
              (`AbilitySystemComponent.BP_ApplyGameplayEffectSpecToTarget` (`AbilitySystemBlueprintLibrary.GetAbilitySystemComponent` (`self.GetAvatarActorFromActorInfo`)) _returnvalue_2 _returnvalue))))))))

(event `WaitCancelInput`
  (`AbilityTask_WaitInputPress.WaitInputPress` false
    (:`OnPress`
      (`self.K2_CancelAbility`))))

(fn `GetTargetGroundLocation`
  (params (AttackTarget :type "Actor Object Reference"))
  (returns (GroundedAttackTarget :type "Vector Structure"))
  (bind _returnvalue (`Actor.K2_GetActorLocation` AttackTarget))
  (bind _outhit (`KismetSystemLibrary.LineTraceSingle` _returnvalue (- _returnvalue (0.0 0.0 9999.0)) "TraceTypeQuery1" false (`|MakeArray` AttackTarget)))
  (return (`.Location` (`GameplayStatics.BreakHitResult` _outhit))))