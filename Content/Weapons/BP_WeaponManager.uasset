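; BP_WeaponManager is a component on BP_Player that equips and unequips weapons, toggling off when the same class is requested again.
; With authority, EquipWeapon spawns the weapon, attaches it to the mesh socket and grants its configured abilities.
; OnRep of EquippedWeapon applies the weapon's anim class and movement properties, or restores defaults cached at BeginPlay.
; UnequipWeapon destroys the weapon, restores those defaults and removes the granted abilities.
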(event `self.ReceiveBeginPlay`
  (bind _charactermovement (`Character.CharacterMovement` (`self.OwningCharacter`)))
  (bind _asbp_player (cast `/Game/GameplayAbilitySystem/Characters/BP_Player` (`self.GetOwner`)))
  (bind _output_get (set `self.OwningCharacter` _asbp_player))
  (set `self.DeafaultAnimClass` (`GameplayStatics.GetObjectClass` (`SkeletalMeshComponent.GetAnimInstance` (`Character.Mesh` _output_get))))
  (set `self.DefaultMovementProperties` (make `/Game/Weapons/Data/S_MovementProperties` (`CharacterMovementComponent.MaxWalkSpeed` _charactermovement) (`CharacterMovementComponent.bOrientRotationToMovement` _charactermovement) (`CharacterMovementComponent.bUseControllerDesiredRotation` _charactermovement))))

(event `EquipWeapon`
  (params (WeaponClass :type "/Game/Weapons/BP_Weapon_Base Class Reference"))
  (`/Engine/EditorBlueprintResources/ActorComponentMacros.Switch Has Authority`
    (:`Authority`
      (`self.OwningCharacter`
        (:`then`
          (if (== (`GameplayStatics.GetObjectClass` (`self.EquippedWeapon`)) WeaponClass)
            (`self.UnequipWeapon`)
            (else
              (`self.UnequipWeapon`)
              (bind _returnvalue (`|SpawnActorFromClass` WeaponClass (`KismetMathLibrary.MakeTransform` (0.0 0.0 0.0)) "Undefined" "MultiplyWithRoot" null (`self.OwningCharacter`)))
              (bind _output_get (set `self.EquippedWeapon` _returnvalue))
              (`Actor.K2_AttachToComponent` _output_get (`Character.Mesh` (`self.OwningCharacter`)) (`.SocketName_6_A493D5214663D153EF8A4E932DFB8A54` (break `/Game/Weapons/Data/S_WeaponConfig` (`/Game/Weapons/BP_Weapon_Base.WeaponConfig` _output_get))) "SnapToTarget" "SnapToTarget" "SnapToTarget" true)
              ; Add Weapon abilities
              (bind _returnvalue_2 (`SCharacterBase.GrantAbilities` (`self.OwningCharacter`) (`.AbilitiesToGrant_4_F253401D47A65F91399DE0A4FC4DEF1A` (break `/Game/Weapons/Data/S_WeaponConfig` (`/Game/Weapons/BP_Weapon_Base.WeaponConfig` (`self.EquippedWeapon`))))))
              (set `self.AbilitiesGrantedByWeapon` _returnvalue_2))))
        (:`else`)))))

(event `SetEquippedWeaponProperties`
  (`SkeletalMeshComponent.SetAnimInstanceClass` (`Character.Mesh` (`self.OwningCharacter`)) (`.AnimClass_10_A06A74C34B0AB02D3D96A69C0F3E38FD` (break `/Game/Weapons/Data/S_WeaponConfig` (`/Game/Weapons/BP_Weapon_Base.WeaponConfig` (`self.EquippedWeapon`)))))
  (`self.SetMovementProperties` (`.MovementProperties_13_8F090DB24543AECDFA666396707FF847` (break `/Game/Weapons/Data/S_WeaponConfig` (`/Game/Weapons/BP_Weapon_Base.WeaponConfig` (`self.EquippedWeapon`))))))

(event `UnequipWeapon`
  (bind _equippedweapon (`self.EquippedWeapon`)
    (:`then`
      (`Actor.K2_DestroyActor` _equippedweapon)
      (set `self.EquippedWeapon` null)
      (`SkeletalMeshComponent.SetAnimInstanceClass` (`Character.Mesh` (`self.OwningCharacter`)) (`self.DeafaultAnimClass`))
      (`self.SetMovementProperties` (`self.DefaultMovementProperties`))
      (`SCharacterBase.RemoveAbilities` (`self.OwningCharacter`) (`self.AbilitiesGrantedByWeapon`))
      (`KismetArrayLibrary.Array_Clear` (`self.AbilitiesGrantedByWeapon`)))
    (:`else`)))

(fn `GetEquippedWeapon`
  (returns (EquippedWeapon :type "/Game/Weapons/BP_Weapon_Base Object Reference"))
  (return (`self.EquippedWeapon`)))

(fn `OnRep_EquippedWeapon`
  (`self.EquippedWeapon`
    (:`then`
      (`self.SetEquippedWeaponProperties`))
    (:`else`
      (`self.SetMovementProperties` (`self.DefaultMovementProperties`))
      (`SkeletalMeshComponent.SetAnimInstanceClass` (`Character.Mesh` (`self.OwningCharacter`)) (`self.DeafaultAnimClass`)))))

(fn `SetMovementProperties`
  (params (MovementProperties :type "/Game/Weapons/Data/S_MovementProperties Structure (by ref)"))
  (bind (_maxwalkspeed _orientrotationtomovement _usecontrollerdesirerotation) (break `/Game/Weapons/Data/S_MovementProperties` MovementProperties))
  (set `CharacterMovementComponent.MaxWalkSpeed` _maxwalkspeed (`Character.CharacterMovement` (`self.OwningCharacter`)))
  (set `CharacterMovementComponent.bOrientRotationToMovement` _orientrotationtomovement (`Character.CharacterMovement` (`self.OwningCharacter`)))
  (set `CharacterMovementComponent.bUseControllerDesiredRotation` _usecontrollerdesirerotation (`Character.CharacterMovement` (`self.OwningCharacter`))))