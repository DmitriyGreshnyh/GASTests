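; Base weapon actor that detects hits during an attack window and applies a Gameplay Ability System effect to the targets.
; HitScanStart stores the effect spec, clears prior hits and enables ticking, while HitScanEnd disables it.
; Each tick sphere-traces for Pawns between two trace points, ignoring the instigator.
; Targets with an ability system component receive the effect once per window.
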(event `HitScan`
  (bind _outhits (`KismetSystemLibrary.SphereTraceMultiForObjects` (`SceneComponent.K2_GetComponentLocation` (`self.TraceStart`)) (`SceneComponent.K2_GetComponentLocation` (`self.TraceEnd`)) (`self.HitScanRadius`) (`|MakeArray` "ObjectTypeQuery3" :!type "EObjectTypeQuery Enum") false (`|MakeArray` (`self.GetInstigator`) :!type "Actor Object Reference") (`self.DrawDebugType`) true (struct :`R` 1.0 :`A` 1.0) (struct :`G` 1.0 :`A` 1.0) 0.1))
  (for _array_element _outhits
    (bind (_bblockinghit _binitialoverlap _time _distance _location _impactpoint _normal _impactnormal _physmat _hitactor) (`GameplayStatics.BreakHitResult` _array_element))
    (bind _returnvalue (`AbilitySystemBlueprintLibrary.GetAbilitySystemComponent` _hitactor))
    (`/Engine/EditorBlueprintResources/StandardMacros.IsValid` _returnvalue
      (:`Is Valid`
        (if (not (`KismetArrayLibrary.Array_Contains` (`self.HitActors`) _hitactor))
          (`KismetArrayLibrary.Array_AddUnique` (`self.HitActors`) _hitactor)
          (`AbilitySystemComponent.BP_ApplyGameplayEffectSpecToSelf` _returnvalue (`self.Effect Spec Handle`)))))))

(event `self.ReceiveTick`
  (params (DeltaSeconds :type "Float (single-precision)"))
  (`self.HitScan`))

(event `HitScanStart`
  (params (EffectSpecHandle :type "GameplayEffectSpecHandle Structure"))
  (set `self.Effect Spec Handle` EffectSpecHandle)
  (`KismetArrayLibrary.Array_Clear` (`self.HitActors`))
  (`self.SetActorTickEnabled` true))

(event `HitScanEnd`
  (`self.SetActorTickEnabled` false))

(fn `UserConstructionScript`)